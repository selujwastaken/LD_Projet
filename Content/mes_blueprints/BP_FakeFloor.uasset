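; BP_FakeFloor is a scalable floor block that can be either solid or a fake that objects pass through.
; When Fake is valid, the cube mesh loses collision and takes the Mi_Fake material; otherwise it keeps query-and-physics collision with the prototype grid material.
; The construction script scales the root from per-axis variables and applies this state in the editor, and BeginPlay repeats the same check at runtime.
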(event EventBeginPlay
  (bind _sm_cube (Variables|Default|GetSM_Cube))
  (Variables|Default|GetFake
    (:then
      (Collision|SetCollisionEnabled _sm_cube "NoCollision")
      (Rendering|Material|SetMaterial _sm_cube 0 "/Game/LevelPrototyping/Materials/Mi_Fake.Mi_Fake"))
    (:else
      (Collision|SetCollisionEnabled _sm_cube "QueryAndPhysics")
      (Rendering|Material|SetMaterial _sm_cube 0 "/Game/LevelPrototyping/Materials/M_PrototypeGrid.M_PrototypeGrid"))))

(fn ConstructionScript
  (bind _sm_cube (Variables|Default|GetSM_Cube))
  (Transformation|SetRelativeScale3D (Variables|Default|GetDefaultSceneRoot) (Math|Vector|MakeVector (Variables|Default|GetNew%20Scale%203D%20X) (Variables|Default|GetNew%20Scale%203D%20Y) (Variables|Default|GetNew%20Scale%203D%20Z)))
  (Variables|Default|GetFake
    (:then
      (Collision|SetCollisionEnabled _sm_cube "NoCollision")
      (Rendering|Material|SetMaterial _sm_cube 0 "/Game/LevelPrototyping/Materials/Mi_Fake.Mi_Fake"))
    (:else
      (Collision|SetCollisionEnabled _sm_cube "QueryAndPhysics")
      (Rendering|Material|SetMaterial _sm_cube 0 "/Game/LevelPrototyping/Materials/M_PrototypeGrid.M_PrototypeGrid"))))