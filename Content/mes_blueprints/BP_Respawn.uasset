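; BP_Respawn is a trigger volume that sends the first-person character back to a respawn point.
; When a BP_FirstPersonCharacter begins overlapping the Box, it teleports to the RespawnPoint's location without sweeping, and its controller's rotation is set to match that point's rotation.
; The construction script sizes the Box from the InBoxExtent variable.
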(event OnComponentBeginOverlap(Box)
  (params (OverlappedComponent :type Primitive%20Component%20Object%20Reference) (OtherActor :type Actor%20Object%20Reference) (OtherComp :type Primitive%20Component%20Object%20Reference) (OtherBodyIndex :type Integer) (bFromSweep :type Boolean) (SweepResult :type Hit%20Result%20Structure%20%28by%20ref%29))
  (bind _respawnpoint (Variables|Default|GetRespawnPoint))
  (bind _asbp_first_person_character (Utilities|Casting|CastToBP_FirstPersonCharacter OtherActor))
  (Transformation|SetActorLocation _asbp_first_person_character (Transformation|GetActorLocation _respawnpoint) false true)
  (Pawn|SetControlRotation (Pawn|GetController _asbp_first_person_character) (Transformation|GetActorRotation _respawnpoint)))

(fn ConstructionScript
  (Components|Box|SetBoxExtent (Variables|Default|GetBox) (Variables|Default|GetIn%20Box%20Extent) true))